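; BP_InputReceiver handles one player's input for joining, team selection and readying up before a match.
; Start asks the game mode to display character select if no menu exists, and left/right inputs cycle the team through that menu widget.
; StartGame marks a player with a chosen team ready and notifies the game mode; unready reverses this.
; SpawnAllPlayers passes index, team and itself to the game mode for spawning, then removes the menu.
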(event `InputAction|Start`
  (params (Key :type "Key Structure"))
  (:`Pressed`
    (`/Engine/EditorBlueprintResources/StandardMacros.IsValid` (`self.CharacterMenuRef`)
      (:`Is Not Valid`
        (message `/Game/Blueprints/BPI_GameMode.DisplayCharacterSelect` (`GameplayStatics.GetGameMode`) (`self.PlayerIndex`))
        (set `self.Selecting Team` true)))))

(event `InputAction|MenuLeft`
  (params (Key :type "Key Structure"))
  (:`Pressed`
    (if (not (`self.ReadyToSpawn`))
      (set `self.TeamIsSelected` true)
      (`/Engine/EditorBlueprintResources/StandardMacros.IsValid` (`self.CharacterMenuRef`)
        (:`Is Valid`
          (bind _teamchoice (`/Game/ThirdPersonBP/Blueprints/UI/WBP_CharacterSelect.SwitchTeam` (`self.CharacterMenuRef`) -1))
          (set `self.Team` _teamchoice))))))

(event `InputAction|MenuRight`
  (params (Key :type "Key Structure"))
  (:`Pressed`
    (if (not (`self.ReadyToSpawn`))
      (set `self.TeamIsSelected` true)
      (`/Engine/EditorBlueprintResources/StandardMacros.IsValid` (`self.CharacterMenuRef`)
        (:`Is Valid`
          (bind _teamchoice (`/Game/ThirdPersonBP/Blueprints/UI/WBP_CharacterSelect.SwitchTeam` (`self.CharacterMenuRef`) 1))
          (set `self.Team` _teamchoice))))))

(event `SpawnAllPlayers`
  (bind _charactermenuref (`self.CharacterMenuRef`))
  (message `/Game/Blueprints/BPI_GameMode.SpawnPlayer` (`GameplayStatics.GetGameMode`) (`self.PlayerIndex`) self (`self.Team`))
  (if (`KismetSystemLibrary.IsValid` _charactermenuref)
    (`Widget.RemoveFromParent` _charactermenuref)))

(event `InputAction|StartGame`
  (params (Key :type "Key Structure"))
  (:`Pressed`
    (if (`self.TeamIsSelected`)
      (set `self.ReadyToSpawn` true)
      (message `/Game/Blueprints/BPI_GameMode.MatchIsReadyToStart` (`GameplayStatics.GetGameMode`) (`self.PlayerIndex`)))))

(event `InputAction|MenuUnreadyToSpawn`
  (params (Key :type "Key Structure"))
  (bind _readytospawn (`self.ReadyToSpawn`))
  (:`Pressed`
    (if _readytospawn
      (set `self.ReadyToSpawn` (not _readytospawn))
      (set `self.Team` (`/Game/ThirdPersonBP/Blueprints/UI/WBP_CharacterSelect.TeamChoice` (`self.CharacterMenuRef`))))))

(fn `UserConstructionScript`)