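; Match manager for a timed two-team puck game with roomba players, scoring a team point whenever the puck passes to a different player.
; BeginPlay caches players by index, finds the puck and creates the scoreboard; Tick feeds it the countdown.
; PuckPossessedByNewPlayer updates scores through IncreaseTeamScore; hold-to-score logic is unused.
; Tick calls MatchOver once time expires, showing the winner or tie, then reloading the level after a delay.
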(event `self.ReceiveBeginPlay`
  (bind _outactors (`GameplayStatics.GetAllActorsOfClass` "/Game/ThirdPersonBP/Blueprints/BP_BallPlayerRoomba.BP_BallPlayerRoomba_C"))
  (for _array_element _outactors
    (`KismetArrayLibrary.Array_Set` (`self.Players`) (`/Game/ThirdPersonBP/Blueprints/BP_BallPlayerRoomba.Index` _array_element) _array_element))
  (bind _returnvalue (`GameplayStatics.GetActorOfClass` "/Game/ThirdPersonBP/Blueprints/BP_Puck.BP_Puck_C"))
  (set `self.Puck` _returnvalue)
  (bind _returnvalue_2 (`|CreateWidget` "/Game/ThirdPersonBP/Blueprints/UI/WBP_Scoreboard.WBP_Scoreboard_C"))
  (`UserWidget.AddToViewport` _returnvalue_2 0)
  (set `self.Scoreboard Reference` _returnvalue_2))

(event `self.ReceiveTick`
  (params (DeltaSeconds :type "Float (single-precision)"))
  (bind _scoreboard_reference (`self.Scoreboard Reference`))
  (bind _output_get (set `self.Match Timer` (- (`self.Match Timer`) DeltaSeconds)))
  (if (>= _output_get 0.0)
    (bind (_remainder _returnvalue) (`KismetMathLibrary.FMod` _output_get 60.0))
    (set `/Game/ThirdPersonBP/Blueprints/UI/WBP_Scoreboard.Match Timer Minutes` (`KismetTextLibrary.Conv_TextToString` (`KismetTextLibrary.Conv_IntToText` _returnvalue false true 2)) _scoreboard_reference)
    (set `/Game/ThirdPersonBP/Blueprints/UI/WBP_Scoreboard.Match Timer Seconds` (`KismetTextLibrary.Conv_TextToString` (`KismetTextLibrary.Conv_IntToText` (`KismetMathLibrary.FTrunc` _remainder) false true 2)) _scoreboard_reference)
    (else
      (`self.Match Over`))))

(event `Match Over`
  (`Widget.RemoveFromParent` (`self.Scoreboard Reference`))
  (bind _returnvalue (`|CreateWidget` "/Game/ThirdPersonBP/Blueprints/UI/WBP_VictoryScreen.WBP_VictoryScreen_C"))
  (set `self.VictoryScreen Reference` _returnvalue)
  (if (>= (`self.TeamRedScore`) (`self.TeamBlueScore`))
    (if (> (`self.TeamRedScore`) (`self.TeamBlueScore`))
      (set `/Game/ThirdPersonBP/Blueprints/UI/WBP_VictoryScreen.VictoryText` "Red Team Wins!" (`self.VictoryScreen Reference`))
      (`UserWidget.AddToViewport` (`self.VictoryScreen Reference`) 0)
      (else
        (set `/Game/ThirdPersonBP/Blueprints/UI/WBP_VictoryScreen.VictoryText` "It's a tie!" (`self.VictoryScreen Reference`))
        (`UserWidget.AddToViewport` (`self.VictoryScreen Reference`) 0)))
    (else
      (set `/Game/ThirdPersonBP/Blueprints/UI/WBP_VictoryScreen.VictoryText` "Blue Wins!" (`self.VictoryScreen Reference`))
      (`UserWidget.AddToViewport` (`self.VictoryScreen Reference`) 0)))
  (set `self.MatchOver` true)
  (`KismetSystemLibrary.Delay` 5.0)
  (message `/Game/Blueprints/BPI_GameMode.PostMatchDestroy` (`GameplayStatics.GetGameMode`))
  (`self.K2_DestroyActor` (`self.Puck`))
  (bind _returnvalue_2 (`GameplayStatics.GetCurrentLevelName` true))
  (`GameplayStatics.OpenLevel` (`KismetStringLibrary.Conv_StringToName` _returnvalue_2)))

(event `PuckPossessedByNewPlayer`
  (bind _possessedbyplayerindex (`/Game/ThirdPersonBP/Blueprints/BP_Puck.PossessedByPlayerIndex` (`self.Puck`)))
  (if (not (`self.MatchOver`))
    (if (!= _possessedbyplayerindex (`self.PreviouslyPossessedBy`))
      (bind _output_get (set `self.PreviouslyPossessedBy` _possessedbyplayerindex))
      (bind _team (`/Game/ThirdPersonBP/Blueprints/BP_BallPlayerRoomba.Team` (`|GetArrayItem` (`self.Players`) _output_get)))
      (if (== _team 1)
        (`KismetSystemLibrary.PrintString` "Team blue received the ball")
        (`self.IncreaseTeamScore` _team)
        (else
          (`KismetSystemLibrary.PrintString` "team red received the ball")
          (`self.IncreaseTeamScore` _team))))))

(fn `IncreaseTeamScore`
  (params (`Team Index` :type Integer))
  (bind _scoreboard_reference (`self.Scoreboard Reference`))
  (if (== `Team Index` 1)
    (bind _result (`/Engine/EditorBlueprintResources/StandardMacros.IncrementInt` (`self.TeamBlueScore`))
      (:`  `
        (set `/Game/ThirdPersonBP/Blueprints/UI/WBP_Scoreboard.New Team Blue Score` _result _scoreboard_reference)))
    (else
      (bind _result_2 (`/Engine/EditorBlueprintResources/StandardMacros.IncrementInt` (`self.TeamRedScore`))
        (:`  `
          (set `/Game/ThirdPersonBP/Blueprints/UI/WBP_Scoreboard.New Team Red Score` _result_2 _scoreboard_reference))))))

(fn `UserConstructionScript`)