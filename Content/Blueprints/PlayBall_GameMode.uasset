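; Game mode for PlayBall, a local multiplayer puck game, running player setup and match start.
; On BeginPlay it creates local players at PlayerStarts ordered by numeric tag, each possessing an input receiver, all viewing one shared BP_Camera, then shows the start menu.
; Receivers get character-select widgets; once team selections are ready, they spawn their players, and the mode spawns a cross-linked match manager and puck.
; SpawnPlayer possesses Roomba pawns pre-match.
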(event `self.ReceiveBeginPlay`
  (bind _outactors (`GameplayStatics.GetAllActorsOfClass` "/Game/Blueprints/BP_Camera.BP_Camera_C"))
  (set `self.CameraRef` (`|GetArrayItem` _outactors))
  (`self.GetPlayerStartPoints`)
  (`self.SpawnInputReceivers`)
  (bind _returnvalue (`|CreateWidget` "/Game/ThirdPersonBP/Blueprints/UI/WBP_PlayerStart.WBP_PlayerStart_C"))
  (bind _output_get (set `self.PlayerMenuWidgetRef` _returnvalue))
  (`UserWidget.AddToViewport` _output_get 0))

(fn `DisplayCharacterSelect`
  (params (CurrentPlayerIndex :type Integer))
  (returns (Return :type Boolean))
  (bind _characterselect (`/Game/ThirdPersonBP/Blueprints/UI/WBP_PlayerStart.AddCharacterSelect` (`self.PlayerMenuWidgetRef`) CurrentPlayerIndex))
  (set `/Game/Blueprints/BP_InputReceiver.CharacterMenuRef` _characterselect (`|GetArrayItem` (`self.PlayerInputReceiverArray`) (`local.CurrentPlayerIndex`)))
  (return false))

(fn `GameStarted`
  (set `self.bIsInGame` true)
  (`/Game/Blueprints/BP_Camera.GameStarted` (`self.CameraRef`) (`self.Players`))
  (`KismetSystemLibrary.PrintString` "Hello"))

(fn `GetIsInGame`
  (returns (IsInGame :type Boolean))
  (return (`self.bIsInGame`)))

(fn `GetPlayerStartPoints`
  (bind _outactors (`GameplayStatics.GetAllActorsOfClass` "/Script/Engine.PlayerStart"))
  (set `self.PlayerStartArray` _outactors))

(fn `MatchIsReadyToStart`
  (params (PlayerIndex :type Integer))
  (returns (Return :type Boolean))
  (locals (AllAvailablePlayersReadyToSpawn :type Boolean :default true) (MatchManagerTransform :type "Transform Structure") (`Puck Spawn Transform` :type "Transform Structure" :default "-220.000000,10.000000,157.000000|0.000000,0.000000,0.000000|0.300000,0.300000,0.300000"))
  (for _array_element (`self.PlayerInputReceiverArray`)
    (if (`/Game/Blueprints/BP_InputReceiver.Selecting Team` _array_element)
      (set `local.AllAvailablePlayersReadyToSpawn` (and (`/Game/Blueprints/BP_InputReceiver.TeamIsSelected` _array_element) (`local.AllAvailablePlayersReadyToSpawn`)))))
  (if (`local.AllAvailablePlayersReadyToSpawn`)
    (for _array_element_2 (`self.PlayerInputReceiverArray`)
      (if (`/Game/Blueprints/BP_InputReceiver.TeamIsSelected` _array_element_2)
        (`/Game/Blueprints/BP_InputReceiver.SpawnAllPlayers` _array_element_2)))
    (set `self.MatchStarted` true)
    (bind _returnvalue (`|SpawnActorFromClass` "/Game/Blueprints/BP_MatchManager.BP_MatchManager_C" (`local.MatchManagerTransform`) "Undefined" "OverrideRootScale" null null))
    (bind _returnvalue_2 (`|SpawnActorFromClass` "/Game/ThirdPersonBP/Blueprints/BP_Puck.BP_Puck_C" (`local.Puck Spawn Transform`) "Undefined" "OverrideRootScale" null null))
    (set `/Game/Blueprints/BP_MatchManager.Puck` _returnvalue_2 _returnvalue)
    (set `/Game/ThirdPersonBP/Blueprints/BP_Puck.MatchManager` _returnvalue _returnvalue_2))
  (return false))

(fn `NameToInt`
  (params (PlayerStart :type "PlayerStart Object Reference"))
  (returns (ReturnValue :type Integer))
  (return (`KismetStringLibrary.Conv_StringToInt` (`KismetStringLibrary.Conv_NameToString` (`PlayerStart.PlayerStartTag` PlayerStart)))))

(fn `RemoveUnusedCameras`
  (bind _outactors (`GameplayStatics.GetAllActorsOfClass` "/Script/Engine.CameraActor"))
  (for _array_element _outactors
    (`self.K2_DestroyActor` _array_element)))

(fn `SpawnInputReceivers`
  (locals (Index :type Integer))
  (bind _returnvalue (`GameplayStatics.GetPlayerController` (`local.Index`)))
  (for (_ _array_index) (`self.PlayerStartArray`)
    (set `local.Index` _array_index)
    (for _array_element (`self.PlayerStartArray`)
      (if (== (`self.NameToInt` _array_element) (`local.Index`))
        (`GameplayStatics.CreatePlayer` -1)
        (bind _returnvalue_2 (`|SpawnActorFromClass` "/Game/Blueprints/BP_InputReceiver.BP_InputReceiver_C" (`self.GetTransform` (`|GetArrayItem` (`self.PlayerStartArray`) (`local.Index`))) "Undefined" "OverrideRootScale" null (`local.Index`) null))
        (`KismetArrayLibrary.Array_AddUnique` (`self.PlayerInputReceiverArray`) _returnvalue_2)
        (`Controller.Possess` _returnvalue _returnvalue_2)
        (`KismetArrayLibrary.Array_AddUnique` (`self.PlayerControllerArray`) _returnvalue)
        (`PlayerController.SetViewTargetWithBlend` (`GameplayStatics.GetPlayerController` (`local.Index`)) (`self.CameraRef`) 0.0 "VTBlend_Linear" 0.0 false)))
    (`self.RemoveUnusedCameras`)))

(fn `SpawnPlayer`
  (params (CurrentPlayerIndex :type Integer) (InputReceiver :type "/Game/Blueprints/BP_InputReceiver Object Reference") (Team :type Integer))
  (returns (Return :type Boolean))
  (if (not (`self.MatchStarted`))
    (bind _returnvalue (`|SpawnActorFromClass` "/Game/ThirdPersonBP/Blueprints/BP_BallPlayerRoomba.BP_BallPlayerRoomba_C" (`self.GetTransform` (`local.InputReceiver`)) "Undefined" "OverrideRootScale" null (`local.CurrentPlayerIndex`) Team null))
    (`KismetArrayLibrary.Array_Add` (`self.Players`))
    (`Controller.Possess` (`GameplayStatics.GetPlayerController` (`local.CurrentPlayerIndex`)) _returnvalue)
    (`PlayerController.SetViewTargetWithBlend` (`GameplayStatics.GetPlayerController` (`local.CurrentPlayerIndex`)) (`self.CameraRef`) 0.0 "VTBlend_Linear" 0.0 false)
    (return false)))

(fn `StartGame`
  (returns (Return :type Boolean))
  (if (>= (`KismetArrayLibrary.Array_Length` (`self.Players`)) (`self.MinPlayers`))
    (`self.GameStarted`)
    (return false)))

(fn `UserConstructionScript`)